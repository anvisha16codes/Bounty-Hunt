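; Multiplayer player state that pushes a player's bounty, name and remaining time to the UI through RepNotify functions.
; Bounty changes refresh the owning controller's character floating info, then the first local controller's HUD bounty.
; Name changes refresh the pawn's floating info, and time changes update the first local controller's HUD timer.
; Each update depends on successful casts, and the event graph holds no active logic.
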(fn `OnRep_BountyNumber`
  (bind _asbp_pc_multiplayer (cast `/Game/Multiplayer/Blueprints/BP_PC_Multiplayer` (`self.GetOwner`)))
  (bind _asbp_character_tps (cast `/Game/Multiplayer/Blueprints/BP_Character_TPS` (`Controller.K2_GetPawn` _asbp_pc_multiplayer)))
  (`/Game/Multiplayer/Blueprints/BP_Character_TPS.Update Floating info` _asbp_character_tps)
  (bind _asbp_pc_multiplayer_2 (cast `/Game/Multiplayer/Blueprints/BP_PC_Multiplayer` (`GameplayStatics.GetPlayerController` 0)))
  (`/Game/Multiplayer/Blueprints/BP_PC_Multiplayer.UpdateHUDbounty` _asbp_pc_multiplayer_2))

(fn `OnRep_NameOfPlayer`
  (bind _asbp_character_tps (cast `/Game/Multiplayer/Blueprints/BP_Character_TPS` (`self.GetPawn`)))
  (`/Game/Multiplayer/Blueprints/BP_Character_TPS.Update Floating info` _asbp_character_tps))

(fn `OnRep_RemainingTime`
  (bind _asbp_pc_multiplayer (cast `/Game/Multiplayer/Blueprints/BP_PC_Multiplayer` (`GameplayStatics.GetPlayerController` 0)))
  (`/Game/Multiplayer/Blueprints/WBP_PlayerHUD.Update Timer` (`/Game/Multiplayer/Blueprints/BP_PC_Multiplayer.HUD_Ref` _asbp_pc_multiplayer) (`KismetMathLibrary.Conv_IntToDouble` (`self.RemainingTime`))))

(fn `UserConstructionScript`)