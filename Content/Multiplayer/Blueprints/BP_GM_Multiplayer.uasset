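; Multiplayer game mode that runs a timed bounty match and picks the winner when time runs out.
; A one-second server timer decrements MatchDuration and copies it to every BP_PS_Multiplayer player state.
; At zero it scans player states for the highest BountyNumber, logging a score line only for each new leader.
; It then creates WBP_EndScreen on the authority side only, with no RPC to clients.
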(event `self.ReceiveBeginPlay`
  (`|ExecutionSequence`
    (:`then_0`
      (bind _outactors (`GameplayStatics.GetAllActorsOfClass` "/Game/Multiplayer/Blueprints/BP_Character_TPS.BP_Character_TPS_C"))
      (for (_array_element _array_index) _outactors
        _))
    (:`then_1`
      (`/Engine/EditorBlueprintResources/ActorMacros.Switch Has Authority`
        (:`Authority`
          (set `self.MatchDuration` (`self.MatchDuration`))
          (`KismetSystemLibrary.K2_SetTimer` null "TickMatchTimer" 1.0 true))))))

(event `TickMatchTimer`
  (bind _matchduration (`self.MatchDuration`))
  (if (> _matchduration 0)
    (set `self.MatchDuration` (- _matchduration 1))
    (bind _outactors (`GameplayStatics.GetAllActorsOfClass` "/Game/Multiplayer/Blueprints/BP_PC_Multiplayer.BP_PC_Multiplayer_C"))
    (for _ _outactors
      (`self.UpdateTimeOnPlayers` (`self.MatchDuration`)))
    (else
      (`self.EventEndMatch`))))

(event `UpdateTimeOnPlayers`
  (params (SecondsRemaining :type Integer))
  (set `self.RemainingTime` SecondsRemaining)
  (for _array_element (`GameStateBase.PlayerArray` (`GameplayStatics.GetGameState`))
    (bind _asbp_ps_multiplayer (cast `/Game/Multiplayer/Blueprints/BP_PS_Multiplayer` _array_element))
    (set `/Game/Multiplayer/Blueprints/BP_PS_Multiplayer.RemainingTime` (`self.MatchDuration`) _asbp_ps_multiplayer)))

(event `EventEndMatch`
  (`/Engine/EditorBlueprintResources/ActorMacros.Switch Has Authority`
    (:`Authority`
      (bind _outactors (`GameplayStatics.GetAllActorsOfClass` "/Game/Multiplayer/Blueprints/BP_PC_Multiplayer.BP_PC_Multiplayer_C"))
      (for _array_element _outactors
        (bind _asbp_ps_multiplayer (cast `/Game/Multiplayer/Blueprints/BP_PS_Multiplayer` (`Controller.PlayerState` _array_element)))
        (bind _bountynumber (`/Game/Multiplayer/Blueprints/BP_PS_Multiplayer.BountyNumber` _asbp_ps_multiplayer))
        (if (> _bountynumber (`self.WinnerScore`))
          (set `self.WinnerScore` _bountynumber)
          (bind _nameofplayer (`/Game/Multiplayer/Blueprints/BP_PS_Multiplayer.NameOfPlayer` _asbp_ps_multiplayer))
          (set `self.WinnerName` _nameofplayer)
          (`KismetArrayLibrary.Array_Add` (`self.ScoreLines`) (`KismetTextLibrary.Conv_TextToString` (`|FormatText` "{0} :{1}" _nameofplayer _bountynumber)))))
      (bind _returnvalue (`|CreateWidget` "/Game/Multiplayer/Blueprints/WBP_EndScreen.WBP_EndScreen_C"))
      (bind _output_get (set `self.EndScreenRef` _returnvalue))
      (`/Game/Multiplayer/Blueprints/WBP_EndScreen.SetWinnerName` _output_get)
      (`/Game/Multiplayer/Blueprints/WBP_EndScreen.SetPlayerScores` _output_get)
      (`UserWidget.AddToViewport` _output_get 0))))

(fn `OnRep_RemainingTime`)

(fn `UserConstructionScript`)