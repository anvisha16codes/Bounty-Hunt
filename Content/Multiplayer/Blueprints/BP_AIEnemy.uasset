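; Multiplayer AI enemy that chases and shoots the player, with a floating name and bounty widget and a HUD bounty update on BeginPlay.
; Pawn sensing triggers an AI move toward player controller 0, then the shoot call.
; The shoot event calls fire and damage events, then checks health.
; At zero health it calls the death event, stops movement and stops brain logic, retrying each tick until the brain component is valid.
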(event `self.PawnSensing.OnSeePawn`
  (params (Pawn :type "Pawn Object Reference"))
  (set `self.IS seeing PLayer` true)
  (`self.Follow Player`))

(event `Follow Player`
  (if (`self.IS seeing PLayer`)
    (`|AIMoveTo` self (0.0 0.0 0.0) (`GameplayStatics.GetPlayerController` 0)
      (:`then`
        (`self.AI_Shoot`)))))

(event `AI_Shoot`
  (if (`self.CanShoot?`)
    (`self.ROS_Fire` (struct))
    (`self.MC_AnyDamage`)
    (if (<= (`self.Health`) 0.0)
      (set `self.Alive?` false)
      (set `self.CanShoot?` false)
      (`self.MC_Death`)
      (`NavMovementInterface.StopActiveMovement` (`self.CharacterMovement`))
      (bind _asaicontroller (cast `AIController` (`self.GetController`)))
      (bind _braincomponent (`AIController.BrainComponent` _asaicontroller :!label _label)
        (:`then`
          (`BrainComponent.StopLogic` _braincomponent "Dead"))
        (:`else`
          (`KismetSystemLibrary.DelayUntilNextTick`)
          (goto _label))))))

(event `self.ReceiveBeginPlay`
  (`parent.ReceiveBeginPlay`)
  (bind _aswbp_floating_info (cast `/Game/Multiplayer/Blueprints/WBP_FloatingInfo` (`WidgetComponent.GetUserWidgetObject` (`self.HeadInfoWidget`))))
  (`/Game/Multiplayer/Blueprints/WBP_FloatingInfo.SetPlayerInfo` _aswbp_floating_info (`self.AI Name`) (`self.Bounty Value`))
  (bind _asbp_pc_multiplayer (cast `/Game/Multiplayer/Blueprints/BP_PC_Multiplayer` (`GameplayStatics.GetPlayerController` 0)))
  (`/Game/Multiplayer/Blueprints/BP_PC_Multiplayer.UpdateHUDbounty` _asbp_pc_multiplayer))

(fn `UserConstructionScript`
  (`parent.UserConstructionScript`))