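; Multiplayer player controller that sets up the local player's crosshair and HUD.
; On BeginPlay the local controller spawns a BP_Crosshair actor and adds WBP_PlayerHUD to the viewport.
; SetCrosshairLocation moves the crosshair actor to the hit location, or to the trace end on a miss.
; BeginPlay also caches player 0's HUD, then UpdateHUDbounty calls UpdateBounty with zero and refreshes its bounty text.
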(event `Set Crosshair Location`
  (params (HIT :type Boolean) (`Hit Location` :type "Vector Structure") (`Trace End` :type "Vector Structure"))
  (if (`self.IsLocalController`)
    (bind _crosshair_widget (`self.Crosshair Widget`)
      (:`then`
        (if HIT
          (`self.K2_SetActorLocation` _crosshair_widget `Hit Location` false false)
          (else
            (`self.K2_SetActorLocation` _crosshair_widget `Trace End` false false))))
      (:`else`))))

(event `self.ReceiveBeginPlay`
  (`|ExecutionSequence`
    (:`then_0`
      (if (`self.IsLocalController`)
        (`|ExecutionSequence`
          (:`then_0`
            (bind _returnvalue (`|SpawnActorFromClass` "/Game/Multiplayer/UI/BP_Crosshair.BP_Crosshair_C" (`KismetMathLibrary.MakeTransform` (0.0 0.0 0.0)) "Undefined" "MultiplyWithRoot" null null))
            (set `self.Crosshair Widget` _returnvalue))
          (:`then_1`
            (bind _returnvalue_2 (`|CreateWidget` "/Game/Multiplayer/Blueprints/WBP_PlayerHUD.WBP_PlayerHUD_C"))
            (bind _output_get (set `self.HUD_Ref` _returnvalue_2))
            (`UserWidget.AddToViewport` _output_get 0)))))
    (:`then_1`
      (bind _asbp_pc_multiplayer (cast `/Game/Multiplayer/Blueprints/BP_PC_Multiplayer` (`GameplayStatics.GetPlayerController` 0)))
      (bind _aswbp_player_hud (cast `/Game/Multiplayer/Blueprints/WBP_PlayerHUD` (`/Game/Multiplayer/Blueprints/BP_PC_Multiplayer.HUD_Ref` _asbp_pc_multiplayer)))
      (set `self.As WBP Player HUD` _aswbp_player_hud)
      (`self.UpdateHUDbounty`))))

(event `UpdateHUDbounty`
  (bind _as_wbp_player_hud (`self.As WBP Player HUD`)
    (:`then`
      (`/Game/Multiplayer/Blueprints/WBP_PlayerHUD.UpdateBounty'` _as_wbp_player_hud 0)
      (bind _bountytext (`/Game/Multiplayer/Blueprints/WBP_PlayerHUD.BountyText` _as_wbp_player_hud))
      (`EditableTextBox.SetText` _bountytext (`|FormatText` "{0}" (`KismetTextLibrary.Conv_ObjectToText` _bountytext))))
    (:`else`)))

(fn `UserConstructionScript`)